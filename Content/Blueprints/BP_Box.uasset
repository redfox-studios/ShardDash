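; BP_Box is a breakable crate that launches the player upward when bounced on and bursts into a random number of Shard pickups or pieces.
; The BoxBounce overlap triggers this only while the player is not touching BoxCollision, whose overlaps set IsTouchingBox.
; DestroyObjects breaks it without the launch, scattering shards within BoxCollision's bounds.
; Crystal, speed, attack and lives functions are default-returning stubs, and the collapse sounds are unwired.
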(event OnComponentBeginOverlap(Boxbounce)
  (params (OverlappedComponent :type Primitive%20Component%20Object%20Reference) (OtherActor :type Actor%20Object%20Reference) (OtherComp :type Primitive%20Component%20Object%20Reference) (OtherBodyIndex :type Integer) (bFromSweep :type Boolean) (SweepResult :type Hit%20Result%20Structure%20%28by%20ref%29))
  (bind _returnvalue (Game|GetPlayerCharacter 0))
  (bind _box_collision (Variables|Default|GetBox%20collision))
  (bind (_origin _boxextent) (Collision|GetComponentBounds _box_collision))
  (if (== OtherActor _returnvalue)
    (if (not (Variables|Default|GetIs%20touching%20box))
      (Character|LaunchCharacter _returnvalue "0.000000,0.000000,1200.000000" false false)
      (for _index (range 0 (Math|Random|RandomInteger 5))
        (Game|SpawnActorfromClass "/Game/Meshes/Pickups/Shard.Shard_C" (Math|Conversions|ToTransform(Vector) (Math|Random|RandomPointinBoundingBox _origin _boxextent)) "Undefined" "MultiplyWithRoot" 0 0))
      (Actor|DestroyActor))))

(event OnComponentBeginOverlap(Boxcollision)
  (params (OverlappedComponent :type Primitive%20Component%20Object%20Reference) (OtherActor :type Actor%20Object%20Reference) (OtherComp :type Primitive%20Component%20Object%20Reference) (OtherBodyIndex :type Integer) (bFromSweep :type Boolean) (SweepResult :type Hit%20Result%20Structure%20%28by%20ref%29))
  (if (== OtherActor (Game|GetPlayerCharacter 0))
    (Variables|Default|SetIs%20touching%20box true)))

(event OnComponentEndOverlap(Boxcollision)
  (params (OverlappedComponent :type Primitive%20Component%20Object%20Reference) (OtherActor :type Actor%20Object%20Reference) (OtherComp :type Primitive%20Component%20Object%20Reference) (OtherBodyIndex :type Integer))
  (if (== OtherActor (Game|GetPlayerCharacter 0))
    (Variables|Default|SetIs%20touching%20box false)))

(event EventDestroyObjects
  (bind _box_collision (Variables|Default|GetBox%20collision))
  (bind (_origin _boxextent) (Collision|GetComponentBounds _box_collision))
  (for _index (range 0 (Math|Random|RandomInteger 5))
    (Game|SpawnActorfromClass "/Game/Meshes/Pickups/Shard.Shard_C" (Math|Conversions|ToTransform(Vector) (Math|Random|RandomPointinBoundingBox _origin _boxextent)) "Undefined" "MultiplyWithRoot" 0 0))
  (Actor|DestroyActor))

(fn ConstructionScript)

(fn HaveEndCrystal?
  (return false))

(fn HaveIceCrystal
  (return false))

(fn HaveJungleCrystal
  (return false))

(fn HaveLavaCrystal
  (return false))

(fn HowFastIsPlayer
  (return 0.0))

(fn IsAtacking?
  (return false))

(fn LoadLives
  (return 0 0))