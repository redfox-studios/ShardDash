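; Falling ice spike hazard that drops when the player walks into its detection box.
; Entering that trigger enables physics simulation on the Cube mesh.
; A second box on the spike sends a kill message to the player on overlap and destroys the actor after any overlap.
; The construction script applies exposed variables to both box sizes and the detection box's position.
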(event OnComponentBeginOverlap(Isplayerinbox)
  (params (OverlappedComponent :type Primitive%20Component%20Object%20Reference) (OtherActor :type Actor%20Object%20Reference) (OtherComp :type Primitive%20Component%20Object%20Reference) (OtherBodyIndex :type Integer) (bFromSweep :type Boolean) (SweepResult :type Hit%20Result%20Structure%20%28by%20ref%29))
  (if (== OtherActor (Game|GetPlayerCharacter 0))
    (Physics|SetSimulatePhysics (Variables|Default|GetCube) true)))

(event OnComponentBeginOverlap(icesikebox)
  (params (OverlappedComponent :type Primitive%20Component%20Object%20Reference) (OtherActor :type Actor%20Object%20Reference) (OtherComp :type Primitive%20Component%20Object%20Reference) (OtherBodyIndex :type Integer) (bFromSweep :type Boolean) (SweepResult :type Hit%20Result%20Structure%20%28by%20ref%29))
  (if (== OtherActor (Game|GetPlayerCharacter 0))
    (Class|Function|KillPlayer(Message) OtherActor))
  (Actor|DestroyActor))

(fn ConstructionScript
  (Components|Box|SetBoxExtent (Variables|Default|GetIs%20player%20in%20box) (Variables|Default|Getis%20player%20in%20box%20size) true)
  (Components|Box|SetBoxExtent (Variables|Default|Getice%20sike%20box) (Variables|Default|Getice%20spike%20box%20size) true)
  (Transformation|SetRelativeLocation (Variables|Default|GetIs%20player%20in%20box) (Variables|Default|Getis%20player%20in%20box%20location) false false))