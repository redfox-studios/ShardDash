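; Teleport trigger that returns the player to the level selection map once they hold the current level's crystal.
; On box overlap by the player character, it checks the level name and asks the player for the jungle crystal on LVL_1, ice on LVL_2, or lava on any other level.
; If that crystal is held, it opens LVL_Selection.
; The construction script sizes the trigger box from the Size variable.
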(event OnComponentBeginOverlap(Box)
  (params (OverlappedComponent :type Primitive%20Component%20Object%20Reference) (OtherActor :type Actor%20Object%20Reference) (OtherComp :type Primitive%20Component%20Object%20Reference) (OtherBodyIndex :type Integer) (bFromSweep :type Boolean) (SweepResult :type Hit%20Result%20Structure%20%28by%20ref%29))
  (bind _returnvalue (Game|GetPlayerCharacter 0))
  (if (== OtherActor (Game|GetPlayerCharacter 0))
    (bind _returnvalue_2 (Game|GetCurrentLevelName true))
    (if (Utilities|Enum|Equal(Enum) _returnvalue_2 "LVL_1")
      (bind _have_jungle_crystal (Class|Function|HaveJungleCrystal(Message) _returnvalue))
      (bind _output_get (Variables|Default|SetHave%20Jungle%20Crystl _have_jungle_crystal))
      (if _output_get
        (Game|OpenLevel(byName) "LVL_Selection"))
      (else
        (bind _returnvalue_3 (Game|GetCurrentLevelName true))
        (if (Utilities|Enum|Equal(Enum) _returnvalue_3 "LVL_2")
          (bind _have_ice_crystsl (Class|Function|HaveIceCrystal(Message) _returnvalue))
          (bind _output_get_2 (Variables|Default|SetHave%20Ice%20Crystal _have_ice_crystsl))
          (if _output_get_2
            (Game|OpenLevel(byName) "LVL_Selection"))
          (else
            (bind _have_lava_crystal (Class|Function|HaveLavaCrystal(Message) _returnvalue))
            (bind _output_get_3 (Variables|Default|SetHave%20Laval%20Crystsô _have_lava_crystal))
            (if _output_get_3
              (Game|OpenLevel(byName) "LVL_Selection"))))))))

(event EventBeginPlay)

(fn ConstructionScript
  (Components|Box|SetBoxExtent (Variables|Default|GetBox) (Variables|Default|GetSize) true))