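; BP_Mask is a mask pickup that notifies the player character and destroys itself when the player overlaps its box.
; Custom events can place its sphere or alternately sample PacaikRef's Sipocka location and lerp the actor between samples.
; The looping timer for that sampling and a sphere bobbing loop are disconnected, and BeginPlay is empty.
; Crystal, speed, attack and saved-lives query functions are stubs returning defaults.
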(event OnComponentBeginOverlap(Box)
  (params (OverlappedComponent :type Primitive%20Component%20Object%20Reference) (OtherActor :type Actor%20Object%20Reference) (OtherComp :type Primitive%20Component%20Object%20Reference) (OtherBodyIndex :type Integer) (bFromSweep :type Boolean) (SweepResult :type Hit%20Result%20Structure%20%28by%20ref%29))
  (if (== OtherActor (Game|GetPlayerCharacter 0))
    (Class|Function|PickupMaks(Message) OtherActor)
    (Actor|DestroyActor)))

(event Custom|Setovanie%20lokacie
  (bind _pacaik_ref (Variables|Default|GetPacaik%20ref))
  (bind _sipocka (Variables|/Game/ThirdPerson/Blueprints/BP_ThirdPersonCharacter.BP_ThirdPersonCharacter_C|GetSipocka _pacaik_ref))
  (bind _returnvalue (Transformation|GetWorldLocation _sipocka))
  (Utilities|FlowControl|FlipFlop
    (:A
      (bind _output_get (Variables|Default|SetPovodna%20pozicia _returnvalue))
      (Development|PrintString "raz sem"))
    (:B
      (bind _output_get_2 (Variables|Default|SetNova%20pozicia _returnvalue))
      (Development|PrintString "raz tam")
      (Transformation|SetActorLocation (Math|Vector|Lerp(Vector) _output_get _output_get_2 0.1) false false))))

(event EventSetMaskLocation
  (params (Nova%20lokacia :type Vector :default "0, 0, 0") (Povodna%20lokacia :type Vector :default "0, 0, 0"))
  (Transformation|SetWorldLocation (Variables|Default|GetSphere) (Math|Vector|Lerp(Vector) Povodna%20lokacia Nova%20lokacia 1.0) false false))

(event EventBeginPlay)

(fn ConstructionScript)

(fn HaveEndCrystal?
  (return false))

(fn HaveIceCrystal
  (return false))

(fn HaveJungleCrystal
  (return false))

(fn HaveLavaCrystal
  (return false))

(fn HowFastIsPlayer
  (return 0.0))

(fn IsAtacking?
  (return false))

(fn LoadLives
  (return 0 0))