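; Bounce crate that releases Shard actors when the player hits its bounce triggers, using up a limited Bounces count.
; BoxBounce launches the player upward and BoxBounceBottom does not; both spawn a shard and destroy the crate once Bounces is zero.
; BoxCollision overlap blocks both triggers while the player touches the box.
; DestroyObjects breaks it immediately with one shard; crystal, attack, speed and save queries are default-value stubs.
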(event OnComponentBeginOverlap(Boxcollision)
  (params (OverlappedComponent :type Primitive%20Component%20Object%20Reference) (OtherActor :type Actor%20Object%20Reference) (OtherComp :type Primitive%20Component%20Object%20Reference) (OtherBodyIndex :type Integer) (bFromSweep :type Boolean) (SweepResult :type Hit%20Result%20Structure%20%28by%20ref%29))
  (if (== OtherActor (Game|GetPlayerCharacter 0))
    (Variables|Default|SetIs%20touching%20box true)))

(event OnComponentEndOverlap(Boxcollision)
  (params (OverlappedComponent :type Primitive%20Component%20Object%20Reference) (OtherActor :type Actor%20Object%20Reference) (OtherComp :type Primitive%20Component%20Object%20Reference) (OtherBodyIndex :type Integer))
  (if (== OtherActor (Game|GetPlayerCharacter 0))
    (Variables|Default|SetIs%20touching%20box false)))

(event OnComponentBeginOverlap(Boxbounce)
  (params (OverlappedComponent :type Primitive%20Component%20Object%20Reference) (OtherActor :type Actor%20Object%20Reference) (OtherComp :type Primitive%20Component%20Object%20Reference) (OtherBodyIndex :type Integer) (bFromSweep :type Boolean) (SweepResult :type Hit%20Result%20Structure%20%28by%20ref%29))
  (bind _returnvalue (Game|GetPlayerCharacter 0))
  (bind _cube (Variables|Default|GetCube))
  (bind _cube_2 (Variables|Default|GetCube))
  (bind _returnvalue_2 (Transformation|GetWorldLocation _cube_2))
  (bind _returnvalue_3 (Transformation|GetWorldLocation _cube))
  (if (== OtherActor _returnvalue)
    (if (not (Variables|Default|GetIs%20touching%20box))
      (if (== (Variables|Default|Getbounces) 0)
        (Game|SpawnActorfromClass "/Game/Meshes/Pickups/Shard.Shard_C" (Math|Transform|MakeTransform (Math|Vector|MakeVector (.x _returnvalue_2) (.y _returnvalue_2) (- (.z _returnvalue_2) 1.8e+02)) "0, 0, 0" "1.000000,1.000000,1.000000") "Undefined" "MultiplyWithRoot" 0 0)
        (Character|LaunchCharacter _returnvalue "0.000000,0.000000,1200.000000" true true)
        (Actor|DestroyActor)
        (else
          (Character|LaunchCharacter _returnvalue "0.000000,0.000000,1200.000000" true true)
          (Utilities|FlowControl|Delay 0.3)
          (Game|SpawnActorfromClass "/Game/Meshes/Pickups/Shard.Shard_C" (Math|Transform|MakeTransform (Math|Vector|MakeVector (.x _returnvalue_3) (.y _returnvalue_3) (+ (.z _returnvalue_3) 2e+02)) "0, 0, 0" "1.000000,1.000000,1.000000") "Undefined" "MultiplyWithRoot" 0 0)
          (Variables|Default|Setbounces (- (Variables|Default|Getbounces) 1))
          (Development|PrintString "objavil sa"))))))

(event OnComponentBeginOverlap(Boxbouncebottom)
  (params (OverlappedComponent :type Primitive%20Component%20Object%20Reference) (OtherActor :type Actor%20Object%20Reference) (OtherComp :type Primitive%20Component%20Object%20Reference) (OtherBodyIndex :type Integer) (bFromSweep :type Boolean) (SweepResult :type Hit%20Result%20Structure%20%28by%20ref%29))
  (bind _cube (Variables|Default|GetCube))
  (bind _cube_2 (Variables|Default|GetCube))
  (bind _returnvalue (Transformation|GetWorldLocation _cube_2))
  (bind _returnvalue_2 (Transformation|GetWorldLocation _cube))
  (if (== OtherActor (Game|GetPlayerCharacter 0))
    (if (not (Variables|Default|GetIs%20touching%20box))
      (if (== (Variables|Default|Getbounces) 0)
        (Game|SpawnActorfromClass "/Game/Meshes/Pickups/Shard.Shard_C" (Math|Transform|MakeTransform (Math|Vector|MakeVector (.x _returnvalue) (.y _returnvalue) (- (.z _returnvalue) 1.8e+02)) "0, 0, 0" "1.000000,1.000000,1.000000") "Undefined" "MultiplyWithRoot" 0 0)
        (Actor|DestroyActor)
        (else
          (Utilities|FlowControl|Delay 0.3)
          (Game|SpawnActorfromClass "/Game/Meshes/Pickups/Shard.Shard_C" (Math|Transform|MakeTransform (Math|Vector|MakeVector (.x _returnvalue_2) (.y _returnvalue_2) (- (.z _returnvalue_2) 1.8e+02)) "0, 0, 0" "1.000000,1.000000,1.000000") "Undefined" "MultiplyWithRoot" 0 0)
          (Variables|Default|Setbounces (- (Variables|Default|Getbounces) 1)))))))

(event EventDestroyObjects
  (bind _box_collision (Variables|Default|GetBox%20collision))
  (bind (_origin _boxextent) (Collision|GetComponentBounds _box_collision))
  (Game|SpawnActorfromClass "/Game/Meshes/Pickups/Shard.Shard_C" (Math|Conversions|ToTransform(Vector) (Math|Random|RandomPointinBoundingBox _origin _boxextent)) "Undefined" "MultiplyWithRoot" 0 0)
  (Actor|DestroyActor))

(fn ConstructionScript)

(fn HaveEndCrystal?
  (return false))

(fn HaveIceCrystal
  (return false))

(fn HaveJungleCrystal
  (return false))

(fn HaveLavaCrystal
  (return false))

(fn HowFastIsPlayer
  (return 0.0))

(fn IsAtacking?
  (return false))

(fn LoadLives
  (return 0 0))