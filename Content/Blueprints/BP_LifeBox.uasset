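; BP_LifeBox is a breakable box that calls AddLifeMessage on the player when destroyed and plays a break sound.
; A "hracik"-tagged component overlapping BoxBounce breaks it and launches the player upward, unless the player is touching BoxCollision, which sets a blocking flag.
; The DestroyObjects event breaks it without the launch.
; The crystal, player-state and save query functions are stubs returning default values.
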(event OnComponentBeginOverlap(Boxcollision)
  (params (OverlappedComponent :type Primitive%20Component%20Object%20Reference) (OtherActor :type Actor%20Object%20Reference) (OtherComp :type Primitive%20Component%20Object%20Reference) (OtherBodyIndex :type Integer) (bFromSweep :type Boolean) (SweepResult :type Hit%20Result%20Structure%20%28by%20ref%29))
  (if (== OtherActor (Game|GetPlayerCharacter 0))
    (Variables|Default|Setis%20touching%20box true)))

(event OnComponentBeginOverlap(Boxbounce)
  (params (OverlappedComponent :type Primitive%20Component%20Object%20Reference) (OtherActor :type Actor%20Object%20Reference) (OtherComp :type Primitive%20Component%20Object%20Reference) (OtherBodyIndex :type Integer) (bFromSweep :type Boolean) (SweepResult :type Hit%20Result%20Structure%20%28by%20ref%29))
  (if true
    (if (Components|ComponentHasTag OtherComp "hracik")
      (if (not (Variables|Default|Getis%20touching%20box))
        (Character|LaunchCharacter (Game|GetPlayerCharacter 0) "0.000000,0.000000,1200.000000" true true)
        (Actor|DestroyActor)
        (Class|Function|AddLife(Message) OtherActor)
        (Audio|PlaySoundatLocation "/Game/Sounds/box-destroy2.box-destroy2" "0, 0, 0" "0, 0, 0" 1.0 1.0 0.0 0 0 0 0)))))

(event OnComponentEndOverlap(Boxcollision)
  (params (OverlappedComponent :type Primitive%20Component%20Object%20Reference) (OtherActor :type Actor%20Object%20Reference) (OtherComp :type Primitive%20Component%20Object%20Reference) (OtherBodyIndex :type Integer))
  (if (== OtherActor (Game|GetPlayerCharacter 0))
    (Variables|Default|Setis%20touching%20box false)))

(event EventDestroyObjects
  (Actor|DestroyActor)
  (Class|Function|AddLife(Message) (Game|GetPlayerCharacter 0))
  (Audio|PlaySoundatLocation "/Game/Sounds/box-destroy2.box-destroy2" "0, 0, 0" "0, 0, 0" 1.0 1.0 0.0 0 0 0 0))

(fn ConstructionScript)

(fn HaveEndCrystal?
  (return false))

(fn HaveIceCrystal
  (return false))

(fn HaveJungleCrystal
  (return false))

(fn HaveLavaCrystal
  (return false))

(fn HowFastIsPlayer
  (return 0.0))

(fn IsAtacking?
  (return false))

(fn IsPlayerAlive?
  (return false))

(fn LoadLives
  (return 0 0))