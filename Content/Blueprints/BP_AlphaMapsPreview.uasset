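; Preview actor that lays out the alpha textures from /Game/550_Alphas/Textures on a grid of mesh tiles.
; The construction script queries the Asset Registry for that folder behind a DoOnce, then calls Generate.
; Generate spawns an XTiles by YTiles grid of static mesh components, each with a dynamic M_AlphaMap instance showing the next texture.
; The Planes array serves only as a running texture index.
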(event EventBeginPlay)

(event Collision|EventActorBeginOverlap
  (params (OtherActor :type Actor%20Object%20Reference)))

(event EventTick
  (params (DeltaSeconds :type Float%20%28single-precision%29)))

(fn ConstructionScript
  (Utilities|FlowControl|DoOnce false
    (:Completed
      (bind _outassetdata (Class|AssetRegistry|GetAssetsbyPath (Class|AssetRegistryHelpers|GetAssetRegistry) "/Game/550_Alphas/Textures" false false))
      (Variables|Default|SetAllTheTextures _outassetdata)
      (CallFunction|Generate))))

(fn Generate
  (bind _defaultsceneroot (Variables|Default|GetDefaultSceneRoot))
  (bind _planes (Variables|Default|GetPlanes))
  (bind _returnvalue (Transformation|GetWorldLocation _defaultsceneroot))
  (Utilities|Array|Clear (Variables|Default|GetPlanes))
  (for _index (range 1 (Variables|Default|GetX_Tiles))
    (for _index_2 (range 1 (Variables|Default|GetY_Tiles))
      (bind _returnvalue_2 (AddComponent|AddStaticMeshComponent false (Math|Transform|MakeTransform (Math|Vector|MakeVector (+ (* _index 100) (.x _returnvalue)) (+ (* _index_2 100) (.y _returnvalue)) (.z _returnvalue)) "0, 0, 0" "1.000000,1.000000,1.000000")))
      (Utilities|Array|Add _planes 1)
      (bind _returnvalue_3 (Rendering|Material|CreateDynamicMaterialInstance _returnvalue_2 0 "/Game/Materials/550_Alphas/M_AlphaMap.M_AlphaMap" "None" :!class /Script/Engine.PrimitiveComponent))
      (bind _astexture_2d (Utilities|Casting|CastToTexture2D (Class|AssetRegistryHelpers|GetAsset (Utilities|Array|Get(acopy) (Variables|Default|GetAllTheTextures) (Utilities|Array|LastIndex _planes)))))
      (Rendering|Material|SetTextureParameterValue _returnvalue_3 "Texture" _astexture_2d))))