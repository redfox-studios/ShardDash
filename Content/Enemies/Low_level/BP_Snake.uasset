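; BP_Snake is a low-level patrolling enemy that kills the player on contact unless they are attacking, and dies when bounced on.
; Its construction script applies per-instance mesh, material, transform, hitboxes and an InterpToMovement path point, while a looping timer flips the mesh yaw 180 degrees.
; Overlapping the bounce box launches the player upward and destroys the snake, unless the kill box has set the touching flag.
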(event OnComponentBeginOverlap(Boxcollision)
  (params (OverlappedComponent :type Primitive%20Component%20Object%20Reference) (OtherActor :type Actor%20Object%20Reference) (OtherComp :type Primitive%20Component%20Object%20Reference) (OtherBodyIndex :type Integer) (bFromSweep :type Boolean) (SweepResult :type Hit%20Result%20Structure%20%28by%20ref%29))
  (if (== OtherActor (Game|GetPlayerCharacter 0))
    (bind _is_atacking (Class|Function|IsAtacking?(Message) OtherActor))
    (if (not _is_atacking)
      (Class|Function|KillPlayer(Message) OtherActor)
      (Variables|Default|Setis%20touching%20box true))))

(event OnComponentBeginOverlap(Boxbounce)
  (params (OverlappedComponent :type Primitive%20Component%20Object%20Reference) (OtherActor :type Actor%20Object%20Reference) (OtherComp :type Primitive%20Component%20Object%20Reference) (OtherBodyIndex :type Integer) (bFromSweep :type Boolean) (SweepResult :type Hit%20Result%20Structure%20%28by%20ref%29))
  (bind _returnvalue (Game|GetPlayerCharacter 0))
  (if (== OtherActor _returnvalue)
    (if (not (Variables|Default|Getis%20touching%20box))
      (Character|LaunchCharacter _returnvalue "0.000000,0.000000,1200.000000" true true)
      (Actor|DestroyActor))))

(event OnComponentEndOverlap(Boxcollision)
  (params (OverlappedComponent :type Primitive%20Component%20Object%20Reference) (OtherActor :type Actor%20Object%20Reference) (OtherComp :type Primitive%20Component%20Object%20Reference) (OtherBodyIndex :type Integer))
  (if (== OtherActor (Game|GetPlayerCharacter 0))
    (Variables|Default|Setis%20touching%20box false)))

(event Custom|rotating
  (bind _skeletalmesh (Variables|Default|GetSkeletalMesh))
  (bind _relativerotation (Variables|/Script/Engine.SceneComponent|GetRelativeRotation _skeletalmesh))
  (Transformation|SetRelativeRotation _skeletalmesh (Math|Rotator|MakeRotator (.roll _relativerotation) (.pitch _relativerotation) (+ (.yaw _relativerotation) 1.8e+02)) false false))

(event EventDestroyObjects
  (Actor|DestroyActor))

(event EventBeginPlay
  (Utilities|Time|SetTimerbyEvent (delegate Custom|rotating) (Variables|Default|Getrychlost%20rotCIE) true)
  (Components|Animation|PlayAnimation (Variables|Default|GetSkeletalMesh) "/Game/Enemies/snake_packed_Anim.snake_packed_Anim" true))

(fn ConstructionScript
  (bind _skeletalmesh (Variables|Default|GetSkeletalMesh))
  (Class|InterptoMovementComponent|AddControlPointPosition (Variables|Default|GetInterpToMovement) (Variables|Default|Getposition) true)
  (Variables|Default|Setrychlost%20rotCIE (Variables|Default|Getrychlost%20rotCIE))
  (Variables|/Script/Engine.InterpToMovementComponent|SetDuration (Variables|Default|GetInterpToMovement) (Variables|Default|Getdurtion))
  (Components|SkeletalMesh|SetSkeletalMeshAsset (Variables|Default|GetSkeletalMesh) (Variables|Default|GetEnemak))
  (Transformation|SetRelativeScale3D _skeletalmesh (Variables|Default|Getvelkost))
  (Rendering|Material|SetMaterial _skeletalmesh 0 (Variables|Default|GetMaterial))
  (Transformation|SetRelativeRotation (Variables|Default|GetSkeletalMesh) (Variables|Default|Getrotation) false false)
  (Components|Box|SetBoxExtent (Variables|Default|GetBox%20collision) (Variables|Default|GetCollision%20box%20size) true)
  (Components|Box|SetBoxExtent (Variables|Default|GetBox%20bounce) (Variables|Default|Getbounce%20box%20size) true)
  (Transformation|SetRelativeLocation (Variables|Default|GetBox%20bounce) (Variables|Default|Getbounce%20box%20location) false false)
  (Transformation|SetRelativeLocation (Variables|Default|GetBox%20collision) (Variables|Default|Getcollision%20box%20location) false false))

(fn HaveEndCrystal?
  (return false))

(fn HaveIceCrystal
  (return false))

(fn HaveJungleCrystal
  (return false))

(fn HaveLavaCrystal
  (return false))

(fn HowFastIsPlayer
  (return 0.0))

(fn IsAtacking?)

(fn LoadLives
  (return 0 0))