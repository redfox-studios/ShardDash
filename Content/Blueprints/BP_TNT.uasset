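; BP_TNT is an explosive TNT actor that kills the player when destroyed.
; DestroyObjects messages player 0 to die, spawns an explosion Niagara effect at the cube, destroys the actor and calls a sound at world origin, with no sound asset shown.
; Box overlaps track PlayerIsIn, but the explosion never checks it, so the kill is unconditional.
; Crystal, speed, attack and lives functions are stubs returning defaults.
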(event OnComponentBeginOverlap(Box)
  (params (OverlappedComponent :type Primitive%20Component%20Object%20Reference) (OtherActor :type Actor%20Object%20Reference) (OtherComp :type Primitive%20Component%20Object%20Reference) (OtherBodyIndex :type Integer) (bFromSweep :type Boolean) (SweepResult :type Hit%20Result%20Structure%20%28by%20ref%29))
  (if (== OtherActor (Game|GetPlayerCharacter 0))
    (Variables|Default|SetPlayer%20is%20in true)))

(event OnComponentEndOverlap(Box)
  (params (OverlappedComponent :type Primitive%20Component%20Object%20Reference) (OtherActor :type Actor%20Object%20Reference) (OtherComp :type Primitive%20Component%20Object%20Reference) (OtherBodyIndex :type Integer))
  (if (== OtherActor (Game|GetPlayerCharacter 0))
    (Variables|Default|SetPlayer%20is%20in false)))

(event EventDestroyObjects
  (Class|Function|KillPlayer(Message) (Game|GetPlayerCharacter 0))
  (Niagara|SpawnSystematLocation "/Game/Particles/Systems/NS_Explosion.NS_Explosion" (Transformation|GetWorldLocation (Variables|Default|GetCube)))
  (Actor|DestroyActor)
  (Audio|PlaySoundatLocation 0 "0, 0, 0" "0, 0, 0" 1.0 1.0 0.0 0 0 0 0))

(fn ConstructionScript)

(fn HaveEndCrystal?
  (return false))

(fn HaveIceCrystal
  (return false))

(fn HaveJungleCrystal
  (return false))

(fn HaveLavaCrystal
  (return false))

(fn HowFastIsPlayer
  (return 0.0))

(fn IsAtacking?
  (return false))

(fn LoadLives
  (return 0 0))