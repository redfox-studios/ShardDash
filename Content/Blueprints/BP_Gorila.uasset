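; BP_Gorila is a gorilla hazard that travels along a spline, killing the player and breaking objects in its path.
; ziskajref receives the spline actor and starts a timeline that moves and rotates the gorilla along it over TimeToComplete.
; Box overlaps send kill or destroy messages to the player or GorilaCanDeystroy-tagged actors.
; A looping timer removes it when the player dies; VypniSaGorila destroys it with an explosion.
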(event OnComponentBeginOverlap(Box)
  (params (OverlappedComponent :type Primitive%20Component%20Object%20Reference) (OtherActor :type Actor%20Object%20Reference) (OtherComp :type Primitive%20Component%20Object%20Reference) (OtherBodyIndex :type Integer) (bFromSweep :type Boolean) (SweepResult :type Hit%20Result%20Structure%20%28by%20ref%29))
  (if (== OtherActor (Game|GetPlayerCharacter 0))
    (Class|Function|GorilaTaZabila(Message) OtherActor)
    (elif (Actor|ActorHasTag OtherActor "GorilaCanDeystroy")
      (Class|Function|DestroyObjects(Message) OtherActor))))

(event Custom|move%20gorila)

(event Custom|ziskajref
  (params (NewParam :type BP%20Autorun%20Object%20Reference))
  (Variables|Default|Setautoranbp NewParam)
  (Components|Timeline|SetPlayRate (Variables|Default|GetT-Move) (/ 1.0 (Variables|Default|Gettime%20to%20complete)))
  (bind _move (Timeline|T-Move PlayFromStart)
    (:Update
      (Transformation|SetActorLocationAndRotation (Spline|GetLocationatDistanceAlongSpline (Variables|/Game/Blueprints/BP_autorun.BP_autorun_C|GetSpline (Variables|Default|Getautoranbp)) (Math|Float|Lerp 0.0 (Spline|GetSplineLength (Variables|/Game/Blueprints/BP_autorun.BP_autorun_C|GetSpline (Variables|Default|Getautoranbp))) _move) "World") (Spline|GetRotationatDistanceAlongSpline (Variables|/Game/Blueprints/BP_autorun.BP_autorun_C|GetSpline (Variables|Default|Getautoranbp)) (Math|Float|Lerp 0.0 (Spline|GetSplineLength (Variables|/Game/Blueprints/BP_autorun.BP_autorun_C|GetSpline (Variables|Default|Getautoranbp))) _move) "World")))))

(event Custom|znicenie%20gorili
  (bind _zomrelino_hracino (Class|Function|IsPlayerAlive?(Message) (Game|GetPlayerCharacter 0)))
  (if (not _zomrelino_hracino)
    (Actor|DestroyActor)))

(event EventSendReferencetoSpline
  (params (reference%20to%20spline :type Spline%20Component%20Object%20Reference)))

(event EventReleaseGorila)

(event EventBeginPlay
  (Utilities|Time|SetTimerbyEvent (delegate Custom|znicenie%20gorili) 1.0 true)
  (Components|Animation|PlayAnimation (Variables|Default|GetSkeletalMesh) "/Game/Enemies/gorila_swim/gorila3__1__Anim_Armature_ArmatureAction.gorila3__1__Anim_Armature_ArmatureAction" true))

(event EventVypniSaGorila
  (Niagara|SpawnSystematLocation "/Game/Particles/Systems/NS_Explosion.NS_Explosion" (Transformation|GetWorldLocation (Variables|Default|GetSkeletalMesh)))
  (Components|DestroyComponent (Variables|Default|GetBox))
  (Actor|DestroyActor))

(fn ConstructionScript
  (Variables|Default|Settime%20to%20complete (Variables|Default|Gettime%20to%20complete)))

(fn HaveEndCrystal?
  (return false))

(fn HaveIceCrystal
  (return false))

(fn HaveJungleCrystal
  (return false))

(fn HaveLavaCrystal
  (return false))

(fn HowFastIsPlayer
  (return 0.0))

(fn IsAtacking?
  (return false))

(fn IsPlayerAlive?)

(fn LoadLives
  (return 0 0))