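; BP_Fence is a fence actor that removes itself from the level when its DestroyObjects event is called.
; That event calls DestroyActor directly, with no effects or conditions.
; The player-related functions for crystals, speed, attacking, alive state and saved lives are stubs returning false or zero, likely from a shared interface.
; The construction script is empty.
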(event EventDestroyObjects
  (Actor|DestroyActor))

(fn ConstructionScript)

(fn HaveEndCrystal?
  (return false))

(fn HaveIceCrystal
  (return false))

(fn HaveJungleCrystal
  (return false))

(fn HaveLavaCrystal
  (return false))

(fn HowFastIsPlayer
  (return 0.0))

(fn IsAtacking?
  (return false))

(fn IsPlayerAlive?
  (return false))

(fn LoadLives
  (return 0 0))