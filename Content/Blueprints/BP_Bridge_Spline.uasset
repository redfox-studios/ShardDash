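; Spline-built bridge that collapses when an actor tagged "Gorila" enters its DestroyingBox trigger.
; The construction script lays a spline mesh along each segment between neighboring spline points and sizes the trigger and spawning boxes from variables.
; On that overlap it scatters BP_Bridge_Plank actors at random points inside SpawningBox, sends VypniSaGorilaMessage to the overlapping actor, then destroys itself.
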(event OnComponentBeginOverlap(Destroyingbox)
  (params (OverlappedComponent :type Primitive%20Component%20Object%20Reference) (OtherActor :type Actor%20Object%20Reference) (OtherComp :type Primitive%20Component%20Object%20Reference) (OtherBodyIndex :type Integer) (bFromSweep :type Boolean) (SweepResult :type Hit%20Result%20Structure%20%28by%20ref%29))
  (bind _spawning_box (Variables|Default|GetSpawning%20box))
  (bind (_origin _boxextent) (Collision|GetComponentBounds _spawning_box))
  (if (Actor|ActorHasTag OtherActor "Gorila")
    (for _index (range 0 10)
      (Game|SpawnActorfromClass "/Game/Blueprints/BP_Bridge_Plank.BP_Bridge_Plank_C" (Math|Transform|MakeTransform (Math|Random|RandomPointinBoundingBox _origin _boxextent) "0, 0, 0" "1.000000,1.000000,1.000000") "Undefined" "MultiplyWithRoot" 0 0))
    (Class|Function|VypniSaGorila(Message) OtherActor)
    (Actor|DestroyActor)))

(fn ConstructionScript
  (bind _spline (Variables|Default|GetSpline))
  (Components|Box|SetBoxExtent (Variables|Default|GetDestroying%20box) (Variables|Default|Getsize) true)
  (Components|Box|SetBoxExtent (Variables|Default|GetSpawning%20box) (Variables|Default|Getsize%20spawning) true)
  (for _index (range 0 (- (Spline|GetNumberOfSplinePoints (Variables|Default|GetSpline)) 2))
    (bind _returnvalue (AddComponent|AddSplineMeshComponent false))
    (SplineMesh|SetStartandEnd _returnvalue (.Location (Spline|GetLocationandTangentatSplinePoint _spline _index "Local")) (.Tangent (Spline|GetLocationandTangentatSplinePoint _spline _index "Local")) (.Location (Spline|GetLocationandTangentatSplinePoint _spline (+ _index 1) "Local")) (.Tangent (Spline|GetLocationandTangentatSplinePoint _spline (+ _index 1) "Local")) true :!class /Script/Engine.SplineMeshComponent)
    (Transformation|AttachComponentToComponent _returnvalue (Variables|Default|GetDefaultSceneRoot) "None" "KeepRelative" "KeepRelative" "KeepRelative" true)))