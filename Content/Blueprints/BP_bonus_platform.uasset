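; Bonus platform that travels along a spline once the player character overlaps its trigger box.
; The overlap sends the player a DisableMovement message, then restarts a timeline with its play rate scaled by TimeToComplete.
; Each timeline update maps the track's alpha to a distance along the spline and moves the cube there in world space, without sweeping.
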(event OnComponentBeginOverlap(Box)
  (params (OverlappedComponent :type Primitive%20Component%20Object%20Reference) (OtherActor :type Actor%20Object%20Reference) (OtherComp :type Primitive%20Component%20Object%20Reference) (OtherBodyIndex :type Integer) (bFromSweep :type Boolean) (SweepResult :type Hit%20Result%20Structure%20%28by%20ref%29))
  (bind _spline (Variables|Default|GetSpline))
  (if (== OtherActor (Game|GetPlayerCharacter 0))
    (Class|Function|DisableMovement(Message) OtherActor)
    (Components|Timeline|SetPlayRate (Variables|Default|GetT_move) (/ 1.0 (Variables|Default|Gettime%20to%20complete)))
    (bind _t_move (Timeline|T_move PlayFromStart)
      (:Update
        (Transformation|SetWorldLocation (Variables|Default|GetCube) (Spline|GetLocationatDistanceAlongSpline _spline (Math|Float|Lerp 0.0 (Spline|GetSplineLength _spline) _t_move) "World") false false)))))

(fn ConstructionScript
  (Variables|Default|Settime%20to%20complete (Variables|Default|Gettime%20to%20complete)))