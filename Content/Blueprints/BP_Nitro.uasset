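; BP_Nitro is an explosive hazard that kills the player and destroys itself.
; Its box overlap detonates only when the player component tagged "hracik" enters and the player's interface-reported speed meets a threshold.
; The DestroyObjects event detonates it unconditionally, spawning the explosion at the cube.
; The overlap path leaves the effect location unset and plays sound at world origin; other interface functions are empty stubs.
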(event OnComponentBeginOverlap(Box)
  (params (OverlappedComponent :type Primitive%20Component%20Object%20Reference) (OtherActor :type Actor%20Object%20Reference) (OtherComp :type Primitive%20Component%20Object%20Reference) (OtherBodyIndex :type Integer) (bFromSweep :type Boolean) (SweepResult :type Hit%20Result%20Structure%20%28by%20ref%29))
  (bind _returnvalue (Game|GetPlayerCharacter 0))
  (if (== OtherActor _returnvalue)
    (if (Components|ComponentHasTag OtherComp "hracik")
      (bind _speed (Class|Function|HowFastIsPlayer(Message) OtherActor))
      (Variables|Default|Setspeed _speed)
      (if (>= (Variables|Default|Getspeed) 3e+02)
        (Class|Function|KillPlayer(Message) _returnvalue)
        (Actor|DestroyActor)
        (Niagara|SpawnSystematLocation "/Game/Particles/Systems/NS_Explosion.NS_Explosion" "0, 0, 0")
        (Audio|SpawnSoundatLocation "/Game/Sounds/explosion1.explosion1" "0, 0, 0" "0, 0, 0" 1.0 1.0 0.0 0 0)))))

(event EventDestroyObjects
  (Class|Function|KillPlayer(Message) (Game|GetPlayerCharacter 0))
  (Development|PrintString "zabilo ma nitro")
  (Niagara|SpawnSystematLocation "/Game/Particles/Systems/NS_Explosion.NS_Explosion" (Transformation|GetWorldLocation (Variables|Default|GetCube)))
  (Actor|DestroyActor))

(fn ConstructionScript)

(fn HaveEndCrystal?
  (return false))

(fn HaveIceCrystal
  (return false))

(fn HaveJungleCrystal
  (return false))

(fn HaveLavaCrystal
  (return false))

(fn HowFastIsPlayer
  (return 0.0))

(fn IsAtacking?
  (return false))

(fn IsPlayerAlive?
  (return false))

(fn LoadLives
  (return 0 0))