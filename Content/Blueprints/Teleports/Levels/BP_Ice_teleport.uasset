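; Teleport actor for the ice level that opens LVL_2 when the player character overlaps its box trigger.
; On BeginPlay it queries the player's HaveIceCrystalMessage and destroys itself if true, so the teleport is absent once the player has the ice crystal.
; The construction script sets the box extent from a Size variable.
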(event OnComponentBeginOverlap(Box)
  (params (OverlappedComponent :type Primitive%20Component%20Object%20Reference) (OtherActor :type Actor%20Object%20Reference) (OtherComp :type Primitive%20Component%20Object%20Reference) (OtherBodyIndex :type Integer) (bFromSweep :type Boolean) (SweepResult :type Hit%20Result%20Structure%20%28by%20ref%29))
  (if (== OtherActor (Game|GetPlayerCharacter 0))
    (Game|OpenLevel(byName) "LVL_2")))

(event EventBeginPlay
  (bind _have_ice_crystsl (Class|Function|HaveIceCrystal(Message) (Game|GetPlayerCharacter 0)))
  (if _have_ice_crystsl
    (Actor|DestroyActor)))

(fn ConstructionScript
  (Components|Box|SetBoxExtent (Variables|Default|GetBox) (Variables|Default|Getsize) true))