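; Level teleport actor for the jungle that opens LVL_1 when the player character overlaps its trigger box.
; On BeginPlay it queries the player for the jungle crystal through a message call and destroys itself if that returns true.
; The construction script sizes the box from the Size variable.
; The crystal, speed, attack and lives functions are stubs returning default values.
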(event OnComponentBeginOverlap(Box)
  (params (OverlappedComponent :type Primitive%20Component%20Object%20Reference) (OtherActor :type Actor%20Object%20Reference) (OtherComp :type Primitive%20Component%20Object%20Reference) (OtherBodyIndex :type Integer) (bFromSweep :type Boolean) (SweepResult :type Hit%20Result%20Structure%20%28by%20ref%29))
  (if (== OtherActor (Game|GetPlayerCharacter 0))
    (Game|OpenLevel(byName) "LVL_1")))

(event EventBeginPlay
  (bind _have_jungle_crystal (Class|Function|HaveJungleCrystal(Message) (Game|GetPlayerCharacter 0)))
  (if _have_jungle_crystal
    (Actor|DestroyActor)))

(fn ConstructionScript
  (Components|Box|SetBoxExtent (Variables|Default|GetBox) (Variables|Default|Getsize) true))

(fn HaveEndCrystal?
  (return false))

(fn HaveIceCrystal
  (return false))

(fn HaveJungleCrystal
  (return false))

(fn HaveLavaCrystal
  (return false))

(fn HowFastIsPlayer
  (return 0.0))

(fn IsAtacking?
  (return false))

(fn LoadLives
  (return 0 0))