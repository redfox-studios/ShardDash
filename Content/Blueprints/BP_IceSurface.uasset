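; BP_IceSurface is a placeable ice patch that makes the player character slide while inside it.
; Box overlap lowers the player's CharacterMovement ground friction and walking braking deceleration, and leaving restores hardcoded normal values rather than saved ones.
; Only player 0's character is affected.
; The construction script sizes the Box and Plane in X and Y from Scale and toggles Plane visibility with ShowPlane.
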(event OnComponentBeginOverlap(Box)
  (params (OverlappedComponent :type Primitive%20Component%20Object%20Reference) (OtherActor :type Actor%20Object%20Reference) (OtherComp :type Primitive%20Component%20Object%20Reference) (OtherBodyIndex :type Integer) (bFromSweep :type Boolean) (SweepResult :type Hit%20Result%20Structure%20%28by%20ref%29))
  (bind _returnvalue (Game|GetPlayerCharacter 0))
  (bind _charactermovement (Variables|/Script/Engine.Character|GetCharacterMovement _returnvalue))
  (if (== OtherActor _returnvalue)
    (Variables|/Script/Engine.CharacterMovementComponent|SetGroundFriction _charactermovement 0.0)
    (Variables|/Script/Engine.CharacterMovementComponent|SetBrakingDecelerationWalking _charactermovement 2e+02)))

(event OnComponentEndOverlap(Box)
  (params (OverlappedComponent :type Primitive%20Component%20Object%20Reference) (OtherActor :type Actor%20Object%20Reference) (OtherComp :type Primitive%20Component%20Object%20Reference) (OtherBodyIndex :type Integer))
  (bind _returnvalue (Game|GetPlayerCharacter 0))
  (bind _charactermovement (Variables|/Script/Engine.Character|GetCharacterMovement _returnvalue))
  (if (== OtherActor _returnvalue)
    (Variables|/Script/Engine.CharacterMovementComponent|SetGroundFriction _charactermovement 8.0)
    (Variables|/Script/Engine.CharacterMovementComponent|SetBrakingDecelerationWalking _charactermovement 2e+03)))

(fn ConstructionScript
  (bind _scale (Variables|Default|GetScale))
  (Rendering|SetVisibility (Variables|Default|GetPlane) (Variables|Default|Getshow%20plane) false)
  (Transformation|SetRelativeScale3D (Variables|Default|GetBox) (Math|Vector|MakeVector _scale _scale 1.0)))