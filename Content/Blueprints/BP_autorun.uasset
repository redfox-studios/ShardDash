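; BP_autorun is a trigger volume that starts auto-run on the player and releases a gorilla, likely for a chase sequence.
; On the player's first overlap it sends an auto-run start message, spawns BP_Gorila at the Arrow, passes it the Spline and releases it.
; Leaving the box sends an auto-run stop message, while a one-time flag blocks repeat starts and spawns.
; The construction script sizes the box from the Size variable.
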(event OnComponentBeginOverlap(Box)
  (params (OverlappedComponent :type Primitive%20Component%20Object%20Reference) (OtherActor :type Actor%20Object%20Reference) (OtherComp :type Primitive%20Component%20Object%20Reference) (OtherBodyIndex :type Integer) (bFromSweep :type Boolean) (SweepResult :type Hit%20Result%20Structure%20%28by%20ref%29))
  (if (== OtherActor (Game|GetPlayerCharacter 0))
    (if (not (Variables|Default|Getwas%20here))
      (Class|Function|AutoRunStart(Message) OtherActor)
      (Variables|Default|Setwas%20here true)
      (bind _returnvalue (Game|SpawnActorfromClass "/Game/Blueprints/BP_Gorila.BP_Gorila_C" (Math|Conversions|ToTransform(Vector) (Transformation|GetWorldLocation (Variables|Default|GetArrow))) "Undefined" "MultiplyWithRoot" 0 0))
      (bind _output_get (Variables|Default|SetGoroôa _returnvalue))
      (Class|Function|SendReferencetoSpline(Message) _output_get (Variables|Default|GetSpline))
      (Class|Function|ReleaseGorila(Message) _output_get))))

(event OnComponentEndOverlap(Box)
  (params (OverlappedComponent :type Primitive%20Component%20Object%20Reference) (OtherActor :type Actor%20Object%20Reference) (OtherComp :type Primitive%20Component%20Object%20Reference) (OtherBodyIndex :type Integer))
  (if (== OtherActor (Game|GetPlayerCharacter 0))
    (Class|Function|AutoRunStop(Message) OtherActor)))

(fn ConstructionScript
  (Components|Box|SetBoxExtent (Variables|Default|GetBox) (Variables|Default|Getsize) true))